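; Tram rail actor that builds a track by repeating a static mesh along the spline of a referenced rails actor.
; Its construction script calls CopyAlongSpline, which derives copy count and spacing from spline length and mesh X bounds.
; Each added mesh component takes the spline's world-space transform at its distance as its relative transform.
; An alternative that stretches a single Rails spline mesh between the spline's endpoints is left disconnected.
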(event `self.ReceiveBeginPlay`)

(fn `copyAlongSpline`
  (bind _returnvalue (`SplineComponent.GetSplineLength` (`/Game/Maks/BP_TramSpline.Spline` (`self.SplineRailsREf`))))
  (bind _returnvalue_2 (/ _returnvalue (* (.x (`.BoxExtent` (`KismetMathLibrary.BreakBoxSphereBounds` (`StaticMesh.GetBounds` (`self.Staticmesh`))))) 2.0)))
  (for _index (range (+ _returnvalue_2 1))
    (bind _returnvalue_3 (`AddComponent|NODE_AddStaticMeshComponent-0` :`RelativeTransform` (`SplineComponent.GetTransformAtDistanceAlongSpline` (`/Game/Maks/BP_TramSpline.Spline` (`self.SplineRailsREf`)) (`KismetMathLibrary.Conv_IntToDouble` (* _index (/ _returnvalue _returnvalue_2))) "World" false)))
    (`StaticMeshComponent.SetStaticMesh` _returnvalue_3 (`self.Staticmesh`))))

(fn `UserConstructionScript`
  (`self.copyAlongSpline`))