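; Actor that lines a spline with procedurally sized BP_Building actors when play begins.
; It derives the building count and even spacing from the spline length and the first base mesh's width plus a margin.
; Each building spawns at its spline transform with a yaw offset, receiving a random height within a range and the flat group, base and roof sets.
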(event `self.ReceiveBeginPlay`
  (`self.start`))

(fn `start`
  (bind _returnvalue (`SplineComponent.GetSplineLength` (`self.Spline`)))
  (bind _returnvalue_2 (`KismetMathLibrary.Round` (/ _returnvalue (+ (* (.x (`.BoxExtent` (`KismetMathLibrary.BreakBoxSphereBounds` (`StaticMesh.GetBounds` (`|GetArrayItem` (`self.FlatBase`)))))) 2.0) (`self.Margin`)))))
  (for _index (range (+ _returnvalue_2 1))
    (bind _returnvalue_3 (`SplineComponent.GetTransformAtDistanceAlongSpline` (`self.Spline`) (* (/ _returnvalue _returnvalue_2) _index) "World" false))
    (`|SpawnActorFromClass` "/Game/Merel/Bleuprints/BP_Building.BP_Building_C" (`KismetMathLibrary.MakeTransform` (.location _returnvalue_3) (`KismetMathLibrary.MakeRotator` (.roll (.rotation _returnvalue_3)) (.pitch (.rotation _returnvalue_3)) (+ (.yaw (.rotation _returnvalue_3)) (`self.RotationZ`)))) "Undefined" "MultiplyWithRoot" null (`KismetMathLibrary.RandomIntegerInRange` (`self.MinHeight`) (`self.MaxHeigh`)) (`self.FlatGroup`) (`self.FlatBase`) (`self.FlatRoof`) null)))

(fn `UserConstructionScript`)