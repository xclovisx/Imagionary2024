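; Tram rail actor that lays a mesh along the spline of a referenced rails actor when play begins.
; BeginPlay divides the spline length into whole mesh-length steps and adds a deformed SplineMeshComponent per step, using local-space points and length-clamped tangents.
; Every segment's start tangent is sampled at distance zero rather than at its own start.
; CopyAlongSpline is an uncalled alternative that places undeformed static mesh copies in world space.
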(event `self.ReceiveBeginPlay`
  (bind _targetspline (`self.TargetSpline`))
  (bind _returnvalue (`SplineComponent.GetSplineLength` (`self.TargetSpline`)))
  (bind _returnvalue_2 (`KismetMathLibrary.FTrunc` (/ _returnvalue (* (.x (`.BoxExtent` (`KismetMathLibrary.BreakBoxSphereBounds` (`StaticMesh.GetBounds` (`self.Staticmesh`))))) 2.0))))
  (set `self.TargetSpline` (`/Game/Maks/BP_TramSpline.Spline` (`self.SplineRailsREf`)))
  (set `self.RailWidthStep` (/ _returnvalue _returnvalue_2))
  (for _index (range (+ _returnvalue_2 1))
    (bind _returnvalue_3 (`AddComponent|NODE_AddSplineMeshComponent-1` :`RelativeTransform` (`KismetMathLibrary.MakeTransform` (`self.K2_GetActorLocation` self))))
    (`SplineMeshComponent.SetForwardAxis` _returnvalue_3 "X" false)
    (`StaticMeshComponent.SetStaticMesh` _returnvalue_3 (`self.Staticmesh`))
    (bind _returnvalue_location (`KismetMathLibrary.BreakTransform` (`SplineComponent.GetTransformAtDistanceAlongSpline` _targetspline (* _index (`self.RailWidthStep`)) "Local" false)))
    (bind _returnvalue_4 (* (+ _index 1) (`self.RailWidthStep`)))
    (bind _returnvalue_location_2 (`KismetMathLibrary.BreakTransform` (`SplineComponent.GetTransformAtDistanceAlongSpline` _targetspline _returnvalue_4 "Local" false)))
    (`SplineMeshComponent.SetStartAndEnd` _returnvalue_3 _returnvalue_location (`KismetMathLibrary.ClampVectorSize` (`SplineComponent.GetTangentAtDistanceAlongSpline` _targetspline 0.0 "Local") 0.0 (`self.RailWidthStep`)) _returnvalue_location_2 (`KismetMathLibrary.ClampVectorSize` (`SplineComponent.GetTangentAtDistanceAlongSpline` _targetspline _returnvalue_4 "Local") 0.0 (`self.RailWidthStep`)) true)))

(fn `copyAlongSpline`
  (bind _returnvalue (`SplineComponent.GetSplineLength` (`/Game/Maks/BP_TramSpline.Spline` (`self.SplineRailsREf`))))
  (bind _returnvalue_2 (/ _returnvalue (* (.x (`.BoxExtent` (`KismetMathLibrary.BreakBoxSphereBounds` (`StaticMesh.GetBounds` (`self.Staticmesh`))))) 2.0)))
  (for _index (range (+ _returnvalue_2 1))
    (bind _returnvalue_3 (`AddComponent|NODE_AddStaticMeshComponent-0` :`RelativeTransform` (`SplineComponent.GetTransformAtDistanceAlongSpline` (`/Game/Maks/BP_TramSpline.Spline` (`self.SplineRailsREf`)) (`KismetMathLibrary.Conv_IntToDouble` (* _index (/ _returnvalue _returnvalue_2))) "World" false)))
    (`StaticMeshComponent.SetStaticMesh` _returnvalue_3 (`self.Staticmesh`))))

(fn `UserConstructionScript`)