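; Spline spawner that places copies of a chosen static mesh at even intervals along the spline of a referenced actor.
; The Construction Script calls CopyAlongSpline, which divides the spline length by the copy count and adds a static mesh component at each step.
; Each component takes the world-space spline transform, plus location and scale offsets, as its relative transform.
; BeginPlay does nothing.
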(event `self.ReceiveBeginPlay`)

(fn `copyAlongSpline`
  (for _index (range (+ (`self.Copies`) 1))
    (bind (_returnvalue_location _returnvalue_rotation _returnvalue_scale) (`KismetMathLibrary.BreakTransform` (`SplineComponent.GetTransformAtDistanceAlongSpline` (`/Game/Maks/BP_TramSpline.Spline` (`self.SplineREf`)) (`KismetMathLibrary.Conv_IntToDouble` (* _index (/ (`SplineComponent.GetSplineLength` (`/Game/Maks/BP_TramSpline.Spline` (`self.SplineREf`))) (`self.Copies`)))) "World" false)))
    (bind _returnvalue (`AddComponent|NODE_AddStaticMeshComponent-0` :`RelativeTransform` (`KismetMathLibrary.MakeTransform` (+ _returnvalue_location (`self.LocationOffset`)) _returnvalue_rotation (+ _returnvalue_scale (`self.ScaleOffset`)))))
    (`StaticMeshComponent.SetStaticMesh` _returnvalue (`self.ObjectToCopy`))))

(fn `UserConstructionScript`
  (`self.copyAlongSpline`))