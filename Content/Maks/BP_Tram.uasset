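; Tram actor that rides along a target rail spline, carrying the player's pawn.
; On BeginPlay it teleports the pawn above its root and attaches it to itself.
; Each Tick it treats Distance as a percentage of spline length, wraps overshoot, and matches the spline's location and rotation.
; The Speed-based advance of Distance is disconnected, and the construction script applies the chosen mesh.
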(event `self.ReceiveBeginPlay`
  (bind _returnvalue (`Controller.K2_GetPawn` (`GameplayStatics.GetPlayerController` 0)))
  (bind (_returnvalue_x _returnvalue_y _returnvalue_z) (`KismetMathLibrary.BreakVector` (`SceneComponent.K2_GetComponentLocation` (`self.DefaultSceneRoot`))))
  (set `self.SplineMaxdistance` (`SplineComponent.GetSplineLength` (`/Game/Maks/BP_TramSpline.Spline` (`self.TargetRails`))))
  (`/Engine/EditorBlueprintResources/StandardMacros.IsValid` _returnvalue
    (:`Is Valid`
      (`self.K2_SetActorLocation` _returnvalue (`KismetMathLibrary.MakeVector` _returnvalue_x _returnvalue_y (+ _returnvalue_z 200.0)) false true)
      (`self.K2_AttachToActor` _returnvalue self "None" "KeepWorld" "KeepWorld" "KeepRelative" false))))

(event `self.ReceiveTick`
  (params (DeltaSeconds :type "Float (single-precision)"))
  (bind _returnvalue (* (`self.Distance`) (`self.PercentageSpline`)))
  (bind _spline (`/Game/Maks/BP_TramSpline.Spline` (`self.TargetRails`)))
  (bind _returnvalue_2 (`SplineComponent.GetSplineLength` _spline))
  (bind (_returnvalue_location _returnvalue_rotation) (`KismetMathLibrary.BreakTransform` (`SplineComponent.GetTransformAtDistanceAlongSpline` _spline (`KismetMathLibrary.SelectFloat` (- _returnvalue (* (`KismetMathLibrary.FFloor` (/ _returnvalue _returnvalue_2)) _returnvalue_2)) _returnvalue (> _returnvalue _returnvalue_2)) "World" false)))
  ;[1 1 1] Get distance
  (`|ExecutionSequence`
    (:`then_0`
      (set `self.PercentageSpline` (/ (`SplineComponent.GetSplineLength` (`/Game/Maks/BP_TramSpline.Spline` (`self.TargetRails`))) 100.0)))
    (:`then_1`
      ;[1 1 1] Move to distance
      (`SceneComponent.K2_SetWorldTransform` (`self.DefaultSceneRoot`) (`KismetMathLibrary.MakeTransform` _returnvalue_location _returnvalue_rotation) false false))))

(fn `UserConstructionScript`
  (`StaticMeshComponent.SetStaticMesh` (`self.Tram`) (`self.Mesh`)))