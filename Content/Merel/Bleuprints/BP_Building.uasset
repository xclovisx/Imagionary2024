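; BP_Building is a procedural building that stacks randomly chosen static mesh pieces up to a target height (HightBuilding).
; The construction script starts with a FlatBase piece, adds FlatGroup floors while the next piece fits, then caps it with a FlatRoof piece.
; Each piece becomes a new component at the running height HuidigeHoogte, which grows by that mesh's bounds height.
; ChooseLayer picks meshes with an unseeded random index, so layouts can change whenever construction reruns.
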(event `self.ReceiveBeginPlay`)

(fn `ChooseLayer`
  (params (BuildingLayer :type "Array of StaticMesh Object Reference"))
  (set `self.SelectedBuilding` (`|GetArrayItem` BuildingLayer (`self.getRandomBuilding` BuildingLayer))))

(fn `getRandomBuilding`
  (params (TargetArray :type "Array of StaticMesh Object Reference (by ref)"))
  (returns (`Mesh index` :type Integer))
  (return (`KismetMathLibrary.RandomInteger` (`KismetArrayLibrary.Array_Length` TargetArray))))

(fn `UserConstructionScript`
  (bind _returnvalue (* (.z (`.BoxExtent` (`KismetMathLibrary.BreakBoxSphereBounds` (`StaticMesh.GetBounds` (`self.SelectedBuilding`))))) 2.0))
  (`self.ChooseLayer` (`self.FlatBase`))
  (while (< (+ (`self.Huidige hoogte`) _returnvalue) (`self.HightBuilding`))
    (if (> _returnvalue 0.0)
      (bind _returnvalue_2 (`AddComponent|NODE_AddStaticMeshComponent-5` :`RelativeTransform` (`KismetMathLibrary.MakeTransform` (`KismetMathLibrary.MakeVector` 0.0 0.0 (`self.Huidige hoogte`))) :!label _label))
      (`StaticMeshComponent.SetStaticMesh` _returnvalue_2 (`self.SelectedBuilding`))
      (set `self.Huidige hoogte` (+ (`self.Huidige hoogte`) _returnvalue))
      (`self.ChooseLayer` (`self.FlatGroup`))))
  (`self.ChooseLayer` (`self.FlatRoof`))
  (goto _label))